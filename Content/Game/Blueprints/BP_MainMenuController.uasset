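; Main menu player controller that spawns the menu widget, shows the cursor and registers the default Enhanced Input mapping context.
; Hold-to-skip inputs drive timelines that fill a skip button progress bar, which resets if the key is released early.
; Completing Skip during the intro movie stops its media and music and opens Level_2D, while completing Exit during the credits removes the credits widget.
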(event Input|EnhancedActionEvents|EnhancedInputActionIA_Exit
  (params (ActionValue :type Boolean) (ElapsedSeconds :type Float%20%28double-precision%29) (TriggeredSeconds :type Float%20%28double-precision%29) (InputAction :type Input%20Action%20Object%20Reference :default "/Game/Game/Blueprints/Input/Actions/IA_Exit.IA_Exit"))
  (:Started
    (Utilities|IsValid (Variables|/Game/Game/Blueprints/UI/Menu/WBP_MainMenu.WBP_MainMenu_C|GetWBP_Credits (Variables|Default|GetWBP_MainMenu))
      (:Is%20Valid
        (bind _skip (Timeline|Timeline PlayFromStart)
          (:Update
            (Default|UpdateProgressBar (Variables|/Game/Game/Blueprints/UI/Menu/WBP_Credits.WBP_Credits_C|GetWBP_SkipButton (Variables|/Game/Game/Blueprints/UI/Menu/WBP_MainMenu.WBP_MainMenu_C|GetWBP_Credits (Variables|Default|GetWBP_MainMenu))) _skip))
          (:Finished
            (Widget|RemovefromParent (Variables|/Game/Game/Blueprints/UI/Menu/WBP_MainMenu.WBP_MainMenu_C|GetWBP_Credits (Variables|Default|GetWBP_MainMenu))))))))
  (:Completed
    (Utilities|IsValid (Variables|/Game/Game/Blueprints/UI/Menu/WBP_MainMenu.WBP_MainMenu_C|GetWBP_Credits (Variables|Default|GetWBP_MainMenu))
      (:Is%20Valid
        (Utilities|FlowControl|Sequence
          (:then_0
            (Timeline|Timeline Stop))
          (:then_1
            (Default|UpdateProgressBar (Variables|/Game/Game/Blueprints/UI/Menu/WBP_Credits.WBP_Credits_C|GetWBP_SkipButton (Variables|/Game/Game/Blueprints/UI/Menu/WBP_MainMenu.WBP_MainMenu_C|GetWBP_Credits (Variables|Default|GetWBP_MainMenu))) 0.0)))))))

(event Input|EnhancedActionEvents|EnhancedInputActionIA_Skip
  (params (ActionValue :type Boolean) (ElapsedSeconds :type Float%20%28double-precision%29) (TriggeredSeconds :type Float%20%28double-precision%29) (InputAction :type Input%20Action%20Object%20Reference :default "/Game/Game/Blueprints/Input/Actions/IA_Skip.IA_Skip"))
  (:Started
    (Utilities|IsValid (Variables|/Game/Game/Blueprints/UI/Menu/WBP_MainMenu.WBP_MainMenu_C|GetWBP_Movie (Variables|Default|GetWBP_MainMenu))
      (:Is%20Valid
        (bind _skip (Timeline|SkipMovieTimeLine PlayFromStart)
          (:Update
            (Default|UpdateProgressBar (Variables|/Game/Game/Blueprints/UI/Movie/WBP_Movie.WBP_Movie_C|GetWBP_SkipButton (Variables|/Game/Game/Blueprints/UI/Menu/WBP_MainMenu.WBP_MainMenu_C|GetWBP_Movie (Variables|Default|GetWBP_MainMenu))) _skip))
          (:Finished
            (Media|MediaPlayer|Close (Variables|/Game/Game/Blueprints/UI/Menu/WBP_MainMenu.WBP_MainMenu_C|GetMediaPlayer (Variables|Default|GetWBP_MainMenu)) :!class /Script/MediaAssets.MediaPlayer)
            (Components|Activation|SetActive (Variables|/Game/Game/Blueprints/UI/Menu/WBP_MainMenu.WBP_MainMenu_C|GetMusicMovie (Variables|Default|GetWBP_MainMenu)) false true)
            (Game|OpenLevel(byObjectReference) "/Game/Game/Blueprints/Maps/Level_2D.Level_2D"))))))
  (:Completed
    (Utilities|IsValid (Variables|/Game/Game/Blueprints/UI/Menu/WBP_MainMenu.WBP_MainMenu_C|GetWBP_Movie (Variables|Default|GetWBP_MainMenu))
      (:Is%20Valid
        (Utilities|FlowControl|Sequence
          (:then_0
            (Timeline|SkipMovieTimeLine Stop))
          (:then_1
            (Default|UpdateProgressBar (Variables|/Game/Game/Blueprints/UI/Movie/WBP_Movie.WBP_Movie_C|GetWBP_SkipButton (Variables|/Game/Game/Blueprints/UI/Menu/WBP_MainMenu.WBP_MainMenu_C|GetWBP_Movie (Variables|Default|GetWBP_MainMenu))) 0.0)))))))

(event EventBeginPlay
  (bind _returnvalue (PlayerController|LocalPlayerSubsystems|GetEnhancedInputLocalPlayerSubsystem))
  (bind _returnvalue_2 (UserInterface|CreateWidget "/Game/Game/Blueprints/UI/Menu/WBP_MainMenu.WBP_MainMenu_C"))
  (bind _output_get (Variables|Default|SetWBP_MainMenu _returnvalue_2))
  (UserInterface|Viewport|AddtoViewport _output_get 0)
  (Variables|/Script/Engine.PlayerController|SetbShowMouseCursor self true)
  (Utilities|IsValid _returnvalue
    (:Is%20Valid
      (Input|AddMappingContext _returnvalue "/Game/Game/Blueprints/Input/IMC_Default.IMC_Default" 0 "(bIgnoreAllPressedKeysUntilRelease=True,bForceImmediately=False,bNotifyUserSettings=False)"))))

(event EventTick
  (params (DeltaSeconds :type Float%20%28single-precision%29)))

(fn ConstructionScript)