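; Player character with a sprite that handles interaction with nearby objects and switching into dialogue.
; An overlap radius tracks BPI_Interactable actors, and completing IA_SetDestination sends InteractMessage to the externally selected one if it is in range.
; Dialogue events toggle input mode and movement, while Tick flips the sprite by horizontal velocity.
; Mapping-context setup and direct IA_Move movement are disconnected and never run.
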(event OnComponentBeginOverlap(InteractionRadius)
  (params (OverlappedComponent :type Primitive%20Component%20Object%20Reference) (OtherActor :type Actor%20Object%20Reference) (OtherComp :type Primitive%20Component%20Object%20Reference) (OtherBodyIndex :type Integer) (bFromSweep :type Boolean) (SweepResult :type Hit%20Result%20Structure%20%28by%20ref%29))
  (if (Utilities|DoesObjectImplementInterface OtherActor "/Game/Game/Blueprints/Interaction/BPI_Interactable.BPI_Interactable_C")
    (Utilities|Array|AddUnique (Variables|Default|GetClosestInteractables) OtherActor)))

(event OnComponentEndOverlap(InteractionRadius)
  (params (OverlappedComponent :type Primitive%20Component%20Object%20Reference) (OtherActor :type Actor%20Object%20Reference) (OtherComp :type Primitive%20Component%20Object%20Reference) (OtherBodyIndex :type Integer))
  (if (Utilities|DoesObjectImplementInterface OtherActor "/Game/Game/Blueprints/Interaction/BPI_Interactable.BPI_Interactable_C")
    (Utilities|Array|RemoveItem (Variables|Default|GetClosestInteractables) OtherActor)))

(event Input|EnhancedActionEvents|EnhancedInputActionIA_SetDestination
  (params (ActionValue :type Boolean) (ElapsedSeconds :type Float%20%28double-precision%29) (TriggeredSeconds :type Float%20%28double-precision%29) (InputAction :type Input%20Action%20Object%20Reference :default "/Game/Game/Blueprints/Input/Actions/IA_SetDestination.IA_SetDestination"))
  (:Completed
    (if (Utilities|Array|ContainsItem (Variables|Default|GetClosestInteractables) (Variables|Default|GetSelectedInteractable))
      (CallFunction|Interactwith))))

(event Input|EnhancedActionEvents|EnhancedInputActionIA_Move
  (params (ActionValue :type Vector%202D%20Structure) (ElapsedSeconds :type Float%20%28double-precision%29) (TriggeredSeconds :type Float%20%28double-precision%29) (InputAction :type Input%20Action%20Object%20Reference :default "/Game/Game/Blueprints/Input/Actions/IA_Move.IA_Move"))
  ;[0.15 0.15 0.15 0.5] Movement
)

(event EventBeginPlay
  ;[0.15 0.15 0.15 0.5] Add Mapping Context
)

(event EventSetInteractable
  (params (Interactable :type Actor%20Object%20Reference))
  (Variables|Default|SetSelectedInteractable Interactable))

(event EventClearInteractable
  (Variables|Default|SetSelectedInteractable 0))

(event EventTick
  (params (DeltaSeconds :type Float%20%28single-precision%29))
  (bind _sprite (Variables|Default|GetSprite))
  (if (> (Math|Vector|VectorLength (Variables|/Script/Engine.MovementComponent|GetVelocity (Variables|Character|GetCharacterMovement))) 0.02)
    (Math|Float|CompareFloat (.x (Class|NavMovementInterface|GetVelocityforNavMovement (Variables|Character|GetCharacterMovement))) 0.0
      (:>
        (Transformation|SetRelativeRotation _sprite "0, 0, 0" false false))
      (:<
        (Transformation|SetRelativeRotation _sprite "0.000000,180.000000,0.000000" false false)))))

(event EventCloseDialogue
  (Input|SetInputModeGameOnly (Game|GetPlayerController 0) true)
  (Components|Activation|Activate (Variables|Character|GetCharacterMovement) false))

(event EventOpenDialogue
  (params (WidgetToFocus :type Widget%20Object%20Reference))
  (Input|SetInputModeGameandUI (Game|GetPlayerController 0) WidgetToFocus "DoNotLock" true true)
  (Components|Activation|Deactivate (Variables|Character|GetCharacterMovement)))

(fn ConstructionScript)

(fn Interactwith
  (Class|BPIInteractable|Interact(Message) (Variables|Default|GetSelectedInteractable) self))