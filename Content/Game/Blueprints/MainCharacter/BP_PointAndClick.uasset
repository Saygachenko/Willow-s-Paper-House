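; BP_PointAndClick is a player controller that moves its pawn with point-and-click input.
; BeginPlay adds the default Enhanced Input mapping context and enables the cursor and mouse-over events.
; Pressing stops current movement, and holding caches the traced cursor location while steering the pawn straight toward it.
; On release or cancel, a press shorter than the threshold uses SimpleMoveToLocation to travel to the cached destination.
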(event Input|EnhancedActionEvents|EnhancedInputActionIA_SetDestination
  (params (ActionValue :type Boolean) (ElapsedSeconds :type Float%20%28double-precision%29) (TriggeredSeconds :type Float%20%28double-precision%29) (InputAction :type Input%20Action%20Object%20Reference :default "/Game/Game/Blueprints/Input/Actions/IA_SetDestination.IA_SetDestination"))
  (bind (_hit _location) (CallFunction|GetLocationUnderCursor))
  ;[0.15 0.15 0.15 0.5] Move to Point
  (:Triggered
    (if _hit
      (bind _output_get (Variables|Input|SetCachedDestination _location))
      (CallFunction|Follow _output_get)))
  (:Started
    (AI|Navigation|StopMovement))
  (:Canceled
    (if (< ElapsedSeconds (Variables|Input|GetPressedThreshold)) :!label _label
      (AI|Navigation|SimpleMovetoLocation self (Variables|Input|GetCachedDestination))))
  (:Completed
    (goto _label)))

(event EventBeginPlay
  (bind _returnvalue (PlayerController|LocalPlayerSubsystems|GetEnhancedInputLocalPlayerSubsystem))
  ;[0.15 0.15 0.15 0.5] Add mapping context
  (Utilities|IsValid _returnvalue
    (:Is%20Valid
      (Input|AddMappingContext _returnvalue "/Game/Game/Blueprints/Input/IMC_Default.IMC_Default" 0 "(bIgnoreAllPressedKeysUntilRelease=True,bForceImmediately=False,bNotifyUserSettings=False)")
      (Variables|Default|SetbShowMouseCursor true)
      (Variables|Default|SetbEnableMouseOverEvents true))))

(fn ConstructionScript)

(fn GetLocationUnderCursor
  (bind _hitresult (Game|Player|GetHitResultUnderCursorbyChannel "TraceTypeQuery1" true))
  (bind (_bblockinghit _binitialoverlap _time _distance _location) (Collision|BreakHitResult _hitresult))
  (return _bblockinghit _location))

(fn Follow
  (params (Location :type Vector))
  (bind _returnvalue (Pawn|GetControlledPawn))
  (Pawn|Input|AddMovementInput _returnvalue (Math|Vector|GetUnitDirection(Vector) (Transformation|GetActorLocation _returnvalue) Location) 1.0 false))