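; Dialogue-driven fetch-quest actor that, despite its cube naming, spawns a BP_Scissors pickup at a fixed location on the "SpawnCube" dialogue trigger.
; Picking up the item changes the dialogue component's starting row to advance the conversation.
; A "GiveCube" trigger removes the quest item from the dialogue instigator's inventory.
; Dialogue event bindings are swapped and released as steps complete, rather than tracking quest state.
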(event EventBeginPlay
  (EventDispatchers|BindEventtoOnDialogueEventTriggered (Variables|Default|GetAC_DialogueBase) (EventDispatchers|CreateEvent :!event SpawnCube)))

(fn ConstructionScript
  (|CallParentFunction))

(fn SpawnCube
  (params (DialogueTrigger :type Name))
  (if (== DialogueTrigger "SpawnCube")
    (bind _returnvalue (Game|SpawnActorfromClass "/Game/Game/Blueprints/Interaction/BP_Scissors.BP_Scissors_C" (Math|Transform|MakeTransform "200.000000,-100.000000,0.000000" "0, 0, 0" "1.000000,1.000000,1.000000") "Undefined" "MultiplyWithRoot" 0 0))
    (EventDispatchers|BindEventtoPickedUp _returnvalue (EventDispatchers|CreateEvent :!event CubePickedUp))
    (EventDispatchers|BindEventtoOnDialogueEventTriggered (Variables|Default|GetAC_DialogueBase) (EventDispatchers|CreateEvent :!event RemoveCube))
    (EventDispatchers|UnbindEventfromOnDialogueEventTriggered (Variables|Default|GetAC_DialogueBase) (EventDispatchers|CreateEvent :!event SpawnCube))))

(fn RemoveCube
  (params (DialogueTrigger :type Name))
  (if (== DialogueTrigger "GiveCube")
    (Class|BPIMainCharacter|RemovefromInventory(Message) (Variables|/Game/Game/Blueprints/Components/AC_DialogueBase.AC_DialogueBase_C|GetInstigator (Variables|Default|GetAC_DialogueBase)) "qitem_0003")
    (EventDispatchers|UnbindEventfromOnDialogueEventTriggered (Variables|Default|GetAC_DialogueBase) (EventDispatchers|CreateEvent :!event RemoveCube))))

(fn CubePickedUp
  (Variables|/Game/Game/Blueprints/Components/AC_DialogueBase.AC_DialogueBase_C|SetStartingRowName (Variables|Default|GetAC_DialogueBase) "2"))