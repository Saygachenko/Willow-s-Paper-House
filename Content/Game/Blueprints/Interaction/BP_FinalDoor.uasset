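; BP_FinalDoor is the game's final door, opened by using a specific inventory item to trigger the ending.
; Interact checks the player's used item, showing dialogue if it is missing or wrong, otherwise consuming it, opening the doors and adding run and noise widgets.
; A timer then leads into the end-game sequence, where the credits animation finishes by loading the main menu.
; Sprite hover drives the interactable message and, once active, the cursor shape.
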(event OnBeginCursorOver(PaperSprite)
  (params (TouchedComponent :type Primitive%20Component%20Object%20Reference))
  (if (Variables|Default|GetbIsActive?)
    (Variables|/Script/Engine.PlayerController|SetCurrentMouseCursor (Game|GetPlayerController 0) "EyeDropper"))
  (Class|BPIMainCharacter|SetInteractable(Message) (Game|GetPlayerCharacter 0) self))

(event OnEndCursorOver(PaperSprite)
  (params (TouchedComponent :type Primitive%20Component%20Object%20Reference))
  (if (Variables|Default|GetbIsActive?)
    (Variables|/Script/Engine.PlayerController|SetCurrentMouseCursor (Game|GetPlayerController 0) "Default"))
  (Class|BPIMainCharacter|ClearInteractable(Message) (Game|GetPlayerCharacter 0)))

(event Custom|END%20GAME
  (bind _returnvalue (Game|ConstructObjectfromClass "/Game/Game/Blueprints/UI/Menu/WBP_Credits.WBP_Credits_C"))
  (UserInterface|Viewport|AddtoViewport _returnvalue 0)
  (UserInterface|Animation|PlayAnimation _returnvalue (Variables|/Game/Game/Blueprints/UI/Menu/WBP_Credits.WBP_Credits_C|GetStart _returnvalue) 0.0 1 "Forward" 1.0 false)
  (Class|UserWidget|BindtoAnimationFinished _returnvalue (Variables|/Game/Game/Blueprints/UI/Menu/WBP_Credits.WBP_Credits_C|GetStart _returnvalue) (delegate Custom|CustomEvent)))

(event Custom|CustomEvent
  (Game|OpenLevel(byObjectReference) "/Game/Game/Blueprints/Maps/Level_MainMenu.Level_MainMenu"))

(event EventInteract
  (params (Instigator :type Actor%20Object%20Reference))
  (bind _ac_dialoguebase (Variables|Default|GetAC_DialogueBase))
  (bind _ac_dialoguebase_2 (Variables|Default|GetAC_DialogueBase))
  (if (not (Variables|Default|GetbIsActive?))
    (bind _asbp_main_character (Utilities|Casting|CastToBP_MainCharacter Instigator))
    (if (Variables|/Game/Game/Blueprints/MainCharacter/BP_MainCharacter.BP_MainCharacter_C|GetbIsUsingItem? _asbp_main_character)
      (if (== (Variables|/Game/Game/Blueprints/Components/BP_InventoryComponent.BP_InventoryComponent_C|GetUsingItemID (Variables|/Game/Game/Blueprints/MainCharacter/BP_MainCharacter.BP_MainCharacter_C|GetBP_InventoryComponent _asbp_main_character)) "qitem_0008")
        (Class|BPIMainCharacter|RemovefromInventory(Message) _asbp_main_character "qitem_0008" false)
        (Variables|Default|SetbIsActive? true)
        (Audio|PlaySound2D (Variables|Default|GetAudio) 1.0 1.0 0.2 0 0)
        (Default|Open (Variables|Default|GetDoors))
        (Utilities|FlowControl|Delay 0.4)
        (bind _returnvalue (Game|ConstructObjectfromClass "/Game/Game/Blueprints/UI/WBP_Run.WBP_Run_C"))
        (UserInterface|Viewport|AddtoViewport _returnvalue 0)
        (bind _returnvalue_2 (Game|ConstructObjectfromClass "/Game/Game/Blueprints/UI/WBP_Noise.WBP_Noise_C"))
        (UserInterface|Viewport|AddtoViewport _returnvalue_2 0)
        (Utilities|Time|SetTimerbyEvent (EventDispatchers|CreateEvent :!event Custom|END%20GAME) 9.0)
        (else
          (Variables|/Game/Game/Blueprints/Components/AC_DialogueBase.AC_DialogueBase_C|SetStartingRowName _ac_dialoguebase "16")
          (Default|OpenConveration _ac_dialoguebase 0.05)))
      (else
        (Variables|/Game/Game/Blueprints/Components/AC_DialogueBase.AC_DialogueBase_C|SetStartingRowName _ac_dialoguebase_2 "15")
        (Default|OpenConveration _ac_dialoguebase_2 0.05 Instigator)))))

(fn ConstructionScript)