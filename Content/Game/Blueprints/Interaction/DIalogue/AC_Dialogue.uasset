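; AC_Dialogue is an actor component that runs data-table-driven conversations through an on-screen dialogue widget.
; OpenConversation creates WBP_Dialogue with itself as owner and adds it to the viewport; CloseConversation removes it and tells the owning actor to close its interaction message.
; Dialogue looks up the current row and loops over its options, updating the widget with speaker, line and a single-option array each pass.
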(event EventBeginPlay)

(event EventTick
  (params (DeltaSeconds :type Float%20%28single-precision%29)))

(fn OpenConversation
  (bind _returnvalue (UserInterface|CreateWidget "/Game/Game/Blueprints/UI/WBP_Dialogue.WBP_Dialogue_C" 0 self))
  (bind _output_get (Variables|Default|SetDialogueWidget _returnvalue))
  (UserInterface|Viewport|AddtoViewport _output_get 0))

(fn CloseConversation
  (Widget|RemovefromParent (Variables|Default|GetDialogueWidget))
  (Class|BPIInteractable|CloseInteraction(Message) (Components|GetOwner)))

(fn Dialogue
  (bind _returnvalue (Utilities|GetDataTableRow (Variables|Default|GetDialogueDatatable) (Variables|Default|GetCurrentRow))
    (:then
      (for _array_element (.DialogueOptions (Utilities|Struct|BreakST_Dialogue _returnvalue))
        (Default|UpdateDialogueText (Variables|Default|GetDialogueWidget) (.DialogueText (Utilities|Struct|BreakST_Dialogue _returnvalue)) (.SpeakerName (Utilities|Struct|BreakST_Dialogue _returnvalue)) (Utilities|Array|MakeArray (.OptionText (Utilities|Struct|BreakST_Dialogue_Option _array_element))))))))