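; BP_Conversant is an interactable actor that opens a dialogue conversation when the Interact event fires.
; It passes the instigator to its ACDialogueBase dialogue, which is given a short delay between letters.
; Hovering the cursor over its Cube switches the player's cursor to crosshairs and sets the player character's interactable message, and leaving restores the default cursor and clears the message.
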(event OnBeginCursorOver(Cube)
  (params (TouchedComponent :type Primitive%20Component%20Object%20Reference))
  (Variables|/Script/Engine.PlayerController|SetCurrentMouseCursor (Game|GetPlayerController 0) "Crosshairs")
  (Class|BPIMainCharacter|SetInteractable(Message) (Game|GetPlayerCharacter 0) self))

(event OnEndCursorOver(Cube)
  (params (TouchedComponent :type Primitive%20Component%20Object%20Reference))
  (Variables|/Script/Engine.PlayerController|SetCurrentMouseCursor (Game|GetPlayerController 0) "Default")
  (Class|BPIMainCharacter|ClearInteractable(Message) (Game|GetPlayerCharacter 0)))

(event EventInteract
  (params (Instigator :type Actor%20Object%20Reference))
  (Default|OpenConveration (Variables|Default|GetAC_DialogueBase) 0.05 Instigator))

(fn ConstructionScript)