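; BP_MouseBed is an interactable sprite object, the mouse bed, that trades an inventory item for another.
; On Interact, if the main character is using item_0001, it adds its own item data component to the inventory, removes item_0001, fires the picked-up call and opens a dialogue conversation.
; Cursor hover over the sprite sets the player's interactable message while the object is active and clears it on exit.
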(event OnBeginCursorOver(PaperSprite)
  (params (TouchedComponent :type Primitive%20Component%20Object%20Reference))
  (if (Variables|Default|GetbIsActive?)
    (Class|BPIMainCharacter|SetInteractable(Message) (Game|GetPlayerCharacter 0) self)))

(event OnEndCursorOver(PaperSprite)
  (params (TouchedComponent :type Primitive%20Component%20Object%20Reference))
  (Class|BPIMainCharacter|ClearInteractable(Message) (Game|GetPlayerCharacter 0)))

(event EventInteract
  (params (Instigator :type Actor%20Object%20Reference))
  (bind _asbp_main_character (Utilities|Casting|CastToBP_MainCharacter Instigator))
  (if (Variables|/Game/Game/Blueprints/MainCharacter/BP_MainCharacter.BP_MainCharacter_C|GetbIsUsingItem? _asbp_main_character)
    (if (== (Variables|/Game/Game/Blueprints/Components/BP_InventoryComponent.BP_InventoryComponent_C|GetUsingItemID (Variables|/Game/Game/Blueprints/MainCharacter/BP_MainCharacter.BP_MainCharacter_C|GetBP_InventoryComponent _asbp_main_character)) "item_0001")
      (Default|AddtoInventory _asbp_main_character (Variables|Default|GetBP_DataItemComponent))
      (Class|BPIMainCharacter|RemovefromInventory(Message) _asbp_main_character "item_0001")
      (Default|CallPickedUp)
      (Default|OpenConveration (Variables|Default|GetAC_DialogueBase) 0.05 Instigator))))

(fn ConstructionScript)