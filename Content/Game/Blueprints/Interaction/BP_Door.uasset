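; BP_Door is an interactable sprite door that moves the player to a new spot, likely another room or screen.
; On Interact, it teleports the BP_MainCharacter instigator to NewPlayerPos and sets that character's camera to NewCameraPos.
; Hovering the sprite swaps the mouse cursor according to IsLeft and registers the door for the player's interactable message, and leaving resets both.
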(event OnBeginCursorOver(PaperSprite)
  (params (TouchedComponent :type Primitive%20Component%20Object%20Reference))
  (bind _returnvalue (Game|GetPlayerController 0))
  (if (Variables|Default|GetbIsLeft)
    (Variables|/Script/Engine.PlayerController|SetCurrentMouseCursor _returnvalue "GrabHandClosed")
    (else
      (Variables|/Script/Engine.PlayerController|SetCurrentMouseCursor _returnvalue "EyeDropper")))
  (Class|BPIMainCharacter|SetInteractable(Message) (Game|GetPlayerCharacter 0) self))

(event OnEndCursorOver(PaperSprite)
  (params (TouchedComponent :type Primitive%20Component%20Object%20Reference))
  (Variables|/Script/Engine.PlayerController|SetCurrentMouseCursor (Game|GetPlayerController 0) "Default")
  (Class|BPIMainCharacter|ClearInteractable(Message) (Game|GetPlayerCharacter 0)))

(event EventInteract
  (params (Instigator :type Actor%20Object%20Reference))
  (bind _asbp_main_character (Utilities|Casting|CastToBP_MainCharacter Instigator))
  (Transformation|SetActorTransform _asbp_main_character (Math|Transform|MakeTransform (Variables|Default|GetNewPlayerPos) "0, 0, 0" "1.000000,1.000000,1.000000") false true)
  (Default|SetCameraPosition _asbp_main_character (Variables|Default|GetNewCameraPos)))

(fn ConstructionScript)