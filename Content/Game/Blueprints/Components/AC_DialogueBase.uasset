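; Dialogue component that runs branching conversations from a Data Table, one row at a time, through a WBP_DialogueDisplay widget.
; Opening creates the widget and notifies the instigator; each row sets text, options, speaker and portraits, and broadcasts any named trigger.
; NextLine follows IDTo unless options await a ChosenOption jump.
; An ending row stores IDTo as the next conversation's start, then closes the widget and notifies the instigator.
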(event Custom|DialogueTrigger
  (params (TriggerName :type Name))
  (if (!= TriggerName "")
    (Default|CallOnDialogueEventTriggered TriggerName)))

(fn OpenConveration
  (params (DelayBetweenLetters :type Float%20%28single-precision%29) (Instigator :type Actor%20Object%20Reference))
  (Utilities|IsValid (Variables|Default|GetDialogueDisplay)
    (:Is%20Not%20Valid
      (bind _returnvalue (UserInterface|CreateWidget "/Game/Game/Blueprints/UI/Dialogue/WBP_DialogueDisplay.WBP_DialogueDisplay_C" 0 DelayBetweenLetters self))
      (bind _output_get (Variables|Default|SetDialogueDisplay _returnvalue))
      (UserInterface|Viewport|AddtoViewport _output_get 0)
      (bind _output_get_2 (Variables|Default|SetInstigator Instigator))
      (Class|BPIMainCharacter|OpenDialogue(Message) _output_get_2 _returnvalue)
      (Variables|Default|SetCurrentRowName (Variables|Default|GetStartingRowName))
      (CallFunction|ProgressDialogue))))

(fn CloseConversation
  (Widget|RemovefromParent (Variables|Default|GetDialogueDisplay))
  (Variables|Default|SetDialogueDisplay 0)
  (Class|BPIMainCharacter|CloseDialogue(Message) (Variables|Default|GetInstigator)))

(fn ProgressDialogue
  (bind _returnvalue (Utilities|GetDataTableRow (Variables|Default|GetDataTable) (Variables|Default|GetCurrentRowName))
    (:then
      (CallFunction|DialogueTrigger (.Trigger (Utilities|Struct|BreakS_Conversation _returnvalue)))
      (Default|SetText (Variables|Default|GetDialogueDisplay) (.Text (Utilities|Struct|BreakS_Conversation _returnvalue)))
      (if (Utilities|Array|IsEmpty (.Options (Utilities|Struct|BreakS_Conversation _returnvalue)))
        _
        (else
          (Default|SetOptions (Variables|Default|GetDialogueDisplay) (.Options (Utilities|Struct|BreakS_Conversation _returnvalue)))))
      (if (.bPlayerSpeaking (Utilities|Struct|BreakS_Conversation _returnvalue))
        (Default|SetSpeaker (Variables|Default|GetDialogueDisplay) "Ти")
        (Default|ShowPlayerPortrait (Variables|Default|GetDialogueDisplay))
        (Default|HideConversantPortrait (Variables|Default|GetDialogueDisplay))
        (else
          (Default|SetSpeaker (Variables|Default|GetDialogueDisplay) (Variables|Default|GetConversantName))
          (Default|HidePlayerPortrait (Variables|Default|GetDialogueDisplay))
          (Default|ShowConversantPortrait (Variables|Default|GetDialogueDisplay)))))))

(fn NextLine
  (bind _returnvalue (Utilities|GetDataTableRow (Variables|Default|GetDataTable) (Variables|Default|GetCurrentRowName))
    (:then
      (if (.bShouldEndDialogue (Utilities|Struct|BreakS_Conversation _returnvalue))
        (Variables|Default|SetStartingRowName (.ID_To (Utilities|Struct|BreakS_Conversation _returnvalue)))
        (CallFunction|CloseConversation)
        (elif (Utilities|Array|IsEmpty (.Options (Utilities|Struct|BreakS_Conversation _returnvalue)))
          (Variables|Default|SetCurrentRowName (.ID_To (Utilities|Struct|BreakS_Conversation _returnvalue)))
          (CallFunction|ProgressDialogue))))))

(fn ChosenOption
  (params (ID_ToGo :type Name))
  (Variables|Default|SetCurrentRowName ID_ToGo)
  (CallFunction|ProgressDialogue))