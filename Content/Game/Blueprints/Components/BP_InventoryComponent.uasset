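; Inventory component that holds the player's items in fixed-size slots, creates the player menu widget and handles adding, removing, using and combining items.
; Adding fills existing stacks up to the DT_Items stack limit, then empty slots, reporting any remainder.
; Combining takes two selections and swaps different items sharing a CombineID for that result item.
; Event dispatchers announce inventory updates, item use, descriptions and warnings, with sound feedback.
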(event Custom|OnPlayerShownDescription
  (params (ItemName :type Text))
  (Default|CallPlayerShownDescription ItemName))

(event Custom|CloseCancelButton
  (params (bIsSuccess :type Boolean))
  (Widget|SetVisibility (Variables|/Game/Game/Blueprints/UI/WBP_PlayerMenu.WBP_PlayerMenu_C|GetWBP_CancelButton (Variables|Inventory|UI|GetWBP_PlayerMenu)) "Collapsed")
  (Variables|Default|SetUsingItemID "None")
  (Variables|/Script/Engine.PlayerController|SetCurrentMouseCursor (Game|GetPlayerController 0) "Default")
  (if bIsSuccess
    (Audio|PlaySound2D "/Game/Game/Assets/Audio/SFX/item_used.item_used" 1.0 1.0 0.0 0 0)
    (else
      (Audio|PlaySound2D "/Game/Game/Assets/Audio/SFX/item_wrong_used.item_wrong_used" 1.0 1.0 0.0 0 0)
      (Default|CallMessageWarning (Variables|Default|GetCombineMessageWarning)))))

(event EventBeginPlay
  (bind _returnvalue (UserInterface|CreateWidget "/Game/Game/Blueprints/UI/WBP_PlayerMenu.WBP_PlayerMenu_C" 0 self))
  (bind _output_get (Variables|Inventory|UI|SetWBP_PlayerMenu _returnvalue))
  (UserInterface|Viewport|AddtoViewport _output_get 0)
  (Utilities|Array|Resize (Variables|Inventory|GetItems) (Variables|Inventory|GetSizeInventory))
  (EventDispatchers|BindEventtoPlayerShownDescription (Variables|Inventory|UI|GetWBP_PlayerMenu) (EventDispatchers|CreateEvent :!event Custom|OnPlayerShownDescription)))

(event Input|KeyboardEvents|1
  (params (Key :type Key%20Structure :default "None")))

(event Input|KeyboardEvents|2
  (params (Key :type Key%20Structure :default "None")))

(event Input|KeyboardEvents|3
  (params (Key :type Key%20Structure :default "None")))

(event Input|KeyboardEvents|4
  (params (Key :type Key%20Structure :default "None")))

(event Input|KeyboardEvents|5
  (params (Key :type Key%20Structure :default "None")))

(fn AddtoInventory
  (params (ID :type Name) (Quantity :type Integer))
  (while (and (> Quantity 0) (not (LocalVariables|GetHasFailed_Local)))
    (bind (_success _indexslot) (Inventory|FindSlot ID))
    (if _success
      (Inventory|AddtoStack _indexslot 1)
      (Math|Integer|DecrementInt Quantity
        (:%20%20
          (Default|CallUpdateInventory ID :!label _label)
          (Audio|PlaySound2D "/Game/Game/Blueprints/Audio/SFX/item_give_Cue.item_give_Cue" 1.0 1.0 0.0 0 0)))
      (else
        (bind _success_2 (Inventory|IsEmptySlot))
        (if _success_2
          (bind _success_3 (Inventory|CreateNewStack ID 1))
          (if _success_3
            (Math|Integer|DecrementInt Quantity
              (:%20%20
                (goto _label)))
            (else
              (LocalVariables|SetHasFailed_Local true)))
          (else
            (LocalVariables|SetHasFailed_Local true))))))
  (return (not (LocalVariables|GetHasFailed_Local)) Quantity))

(fn FindSlot
  (params (ID :type Name))
  (for (_array_element _array_index) (Variables|Inventory|GetItems)
    (if (== (.ID (Utilities|Struct|BreakFSlotItem _array_element)) ID)
      (if (< (.Quantity (Utilities|Struct|BreakFSlotItem _array_element)) (Inventory|GetMaxSizeSlot ID))
        (return true _array_index))))
  (return false -1))

(fn GetMaxSizeSlot
  (params (ID :type Name))
  (bind _returnvalue (Utilities|GetDataTableRow "/Game/Game/Blueprints/Data/Inventory/DT_Items.DT_Items" ID)
    (:then
      (return (Utilities|Struct|BreakFInfoItem _returnvalue)))
    (:RowNotFound
      (return -1))))

(fn CreateNewStack
  (params (Slot :type Name) (Quantity :type Integer))
  (bind (_success _indexslot) (Inventory|IsEmptySlot))
  (if _success
    (Utilities|Array|SetArrayElem (Variables|Inventory|GetItems) _indexslot (Utilities|Struct|MakeFSlotItem Slot Quantity))
    (return true)
    (else
      (return false))))

(fn AddtoStack
  (params (IndexSlot :type Integer) (Quantity :type Integer))
  (bind _items (Variables|Inventory|GetItems))
  (bind _output (Utilities|Array|Get(acopy) _items IndexSlot))
  (bind (_id _quantity) (Utilities|Struct|BreakFSlotItem _output))
  (Utilities|Array|SetArrayElem (Variables|Inventory|GetItems) IndexSlot (Utilities|Struct|MakeFSlotItem _id (+ _quantity Quantity))))

(fn RemovefromSlot
  (params (Index :type Integer) (RemoveStack :type Boolean))
  (bind _items (Variables|Inventory|GetItems))
  (bind _output (Utilities|Array|Get(acopy) _items Index))
  (bind _quantity (Utilities|Struct|BreakFSlotItem _output))
  (if RemoveStack
    (Utilities|Array|SetArrayElem (Variables|Inventory|GetItems) Index (Utilities|Struct|MakeFSlotItem "" 0))
    (else
      (if (<= _quantity 1)
        (Utilities|Array|SetArrayElem (Variables|Inventory|GetItems) Index (Utilities|Struct|MakeFSlotItem "" 0))
        (else
          (bind _result (Math|Integer|DecrementInt _quantity)
            (:%20%20
              (Utilities|Struct|SetmembersinFSlotItem (Utilities|Array|Get(acopy) (Variables|Inventory|GetItems) Index) _result)))))
      (Default|CallUpdateInventory))))

(fn GetDataItem
  (params (ID :type Name))
  (bind _returnvalue (Utilities|GetDataTableRow "/Game/Game/Blueprints/Data/Inventory/DT_Items.DT_Items" ID)
    (:then
      (return _returnvalue))))

(fn CombineItems
  (params (Index :type Integer))
  (if (!= (Variables|Default|GetLastSelectedIndex) -1)
    (bind _output_get (LocalVariables|SetLastSelectedIndex_Local Index))
    (if (Math|Boolean|ANDBoolean (== (.CombineID (Utilities|Struct|BreakFInfoItem (Inventory|GetDataItem (Utilities|Struct|BreakFSlotItem (Utilities|Array|Get(acopy) (Variables|Inventory|GetItems) _output_get))))) (.CombineID (Utilities|Struct|BreakFInfoItem (Inventory|GetDataItem (Utilities|Struct|BreakFSlotItem (Utilities|Array|Get(acopy) (Variables|Inventory|GetItems) (Variables|Default|GetLastSelectedIndex))))))) (!= (Variables|Default|GetLastSelectedIndex) (LocalVariables|GetLastSelectedIndex_Local)) (!= (Class|KismetMathLibrary|AndIntInt (Utilities|Struct|BreakFSlotItem (Utilities|Array|Get(acopy) (Variables|Inventory|GetItems) (LocalVariables|GetLastSelectedIndex_Local))) (Utilities|Struct|BreakFSlotItem (Utilities|Array|Get(acopy) (Variables|Inventory|GetItems) (Variables|Default|GetLastSelectedIndex)))) 0) (!= (Utilities|Struct|BreakFSlotItem (Utilities|Array|Get(acopy) (Variables|Inventory|GetItems) (LocalVariables|GetLastSelectedIndex_Local))) (Utilities|Struct|BreakFSlotItem (Utilities|Array|Get(acopy) (Variables|Inventory|GetItems) (Variables|Default|GetLastSelectedIndex)))) (and (!= (.CombineID (Utilities|Struct|BreakFInfoItem (Inventory|GetDataItem (Utilities|Struct|BreakFSlotItem (Utilities|Array|Get(acopy) (Variables|Inventory|GetItems) (LocalVariables|GetLastSelectedIndex_Local)))))) "") (!= (.CombineID (Utilities|Struct|BreakFInfoItem (Inventory|GetDataItem (Utilities|Struct|BreakFSlotItem (Utilities|Array|Get(acopy) (Variables|Inventory|GetItems) (Variables|Default|GetLastSelectedIndex)))))) "")))
      (Utilities|FlowControl|Sequence
        (:then_0
          (Inventory|RemovefromSlot (LocalVariables|GetLastSelectedIndex_Local) false))
        (:then_1
          (bind _success (Inventory|AddtoInventory (.CombineID (Utilities|Struct|BreakFInfoItem (Inventory|GetDataItem (Utilities|Struct|BreakFSlotItem (Utilities|Array|Get(acopy) (Variables|Inventory|GetItems) (Variables|Default|GetLastSelectedIndex)))))) 1))
          (if _success
            _
            (else
              _))
          (Inventory|RemovefromSlot (Variables|Default|GetLastSelectedIndex) false)
          (Variables|Default|SetLastSelectedIndex -1)
          (Audio|PlaySound2D "/Game/Game/Blueprints/Audio/SFX/item_combing_Cue.item_combing_Cue" 1.0 1.0 0.0 0 0)
          (return true)))
      (else
        (Variables|Default|SetLastSelectedIndex -1)
        (Default|CallMessageWarning (Variables|Default|GetCombineMessageWarning))
        (Audio|PlaySound2D "/Game/Game/Blueprints/Audio/SFX/item_wrong_used_Cue.item_wrong_used_Cue" 1.0 1.0 0.0 0 0)
        (return true)))
    (else
      (Variables|Default|SetLastSelectedIndex Index)
      (return false))))

(fn IsEmptySlot
  (for (_array_element _array_index) (Variables|Inventory|GetItems)
    (if (== (Utilities|Struct|BreakFSlotItem _array_element) 0)
      (return true _array_index)))
  (return false -1))

(fn GetItemIndex
  (params (ID :type Name))
  (for (_array_element _array_index) (Variables|Inventory|GetItems)
    (if (== (Utilities|Struct|BreakFSlotItem _array_element) ID)
      (return _array_index)
      (else
        (Development|PrintString "There's no such ID in the inventory!")))))

(fn ClearMessage
  (Default|CallMessageWarning))

(fn CancelLastSelectedIndex
  (Variables|Default|SetLastSelectedIndex -1))

(fn UseItem
  (params (ID :type Name))
  (Variables|Default|SetUsingItemID ID)
  (Default|CallUsingItem (Variables|Default|GetUsingItemID)))

(fn FindItem
  (params (Id :type Name))
  (bind _array_element (Utilities|Array|ForEachLoopwithBreak (Variables|Inventory|GetItems))
    (:LoopBody
      (if (== (Utilities|Struct|BreakFSlotItem _array_element) Id)
        (return true)))
    (:Completed
      (return false))))