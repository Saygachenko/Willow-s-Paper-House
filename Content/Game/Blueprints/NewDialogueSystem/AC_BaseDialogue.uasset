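; Dialogue component that runs conversations by starting a StateTree and driving a dialogue widget obtained from the player character.
; Lines and choices come from DataTables by row name; lines play in sequence with a shown-all callback, while choices become BP_BasicChoice objects that report the picked ID.
; DAHolder supplies speaker names, status-based portraits and story progression tags.
; It also tracks asked questions for checks.
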(fn OpenConversation
  (params (StateTreeComponent :type State%20Tree%20Component%20Object%20Reference))
  (Variables|Default|GetDialogueDisplay
    (:then)
    (:else
      (Variables|Default|SetStateTreeComponent StateTreeComponent)
      (bind _dialoguewidget (Class|BPIMainCharacter|GetDialogueWidget(Message) (Game|GetPlayerCharacter 0)))
      (bind _output_get (Variables|Default|SetDialogueDisplay _dialoguewidget))
      (Variables|/Game/Game/Blueprints/UI/Dialogue/WBP_DialogueDisplay.WBP_DialogueDisplay_C|SetTestOwningObject _output_get self)
      (bind _output_get_2 (Variables|Default|SetInstigator (Game|GetPlayerCharacter 0)))
      (Class|BPIMainCharacter|OpenDialogue(Message) _output_get_2 _output_get)
      (AI|Logic|StartLogic (Variables|Default|GetStateTreeComponent)))))

(fn CloseConversation
  (Variables|Default|SetDialogueDisplay 0)
  (Class|BPIMainCharacter|CloseDialogue(Message) (Variables|Default|GetInstigator)))

(fn ShowDialogueLine
  (params (DialogueLine :type ST%20Dialogue%20Structure))
  (bind (_speaker _dialogueline) (Utilities|Struct|BreakST_Dialogue DialogueLine))
  (bind _daholder (Variables|Default|GetDAHolder))
  (bind _currentcharacterstatus (Variables|Default|GetCurrentCharacterStatus))
  (bind _characterda (Default|GetSpeakerDA _daholder _speaker))
  (bind _portrait (Default|GetCharacterPortrait _characterda _currentcharacterstatus))
  (Default|SetText (Variables|Default|GetDialogueDisplay) _dialogueline)
  (Default|SetSpeaker (Variables|Default|GetDialogueDisplay) (Variables|/Game/Game/Blueprints/Dialogues/CharactersDataAssets/DA_Speaker.DA_Speaker_C|GetSpeakerName _characterda))
  (if (Variables|/Game/Game/Blueprints/Dialogues/CharactersDataAssets/DA_Speaker.DA_Speaker_C|GetbIsMainCharacter _characterda)
    (CallFunction|ShowPlayerPortrait _portrait)
    (else
      (CallFunction|ShowConversantPortrait _portrait))))

(fn ShowDialogueLinesfromDataTable
  (params (LineNames :type Array%20of%20Names))
  (Variables|Default|SetLineNamesToShow LineNames)
  (Variables|Default|SetCurrentLineNumber -1)
  (CallFunction|NextLine))

(fn NextLine
  (bind _result (Math|Integer|IncrementInt (Variables|Default|GetCurrentLineNumber))
    (:%20%20
      (if (>= _result (Utilities|Array|Length (Variables|Default|GetLineNamesToShow)))
        (Default|CallShownAllDialogueLines)
        (else
          (bind _returnvalue (Utilities|GetDataTableRow (Variables|Default|GetDialogueDataTable) (Utilities|Array|Get(acopy) (Variables|Default|GetLineNamesToShow) (Variables|Default|GetCurrentLineNumber)))
            (:then
              (CallFunction|ShowDialogueLine _returnvalue))
            (:RowNotFound
              (Default|CallShownAllDialogueLines))))))))

(fn ShowOptions
  (params (Options :type Array%20of%20BP%20Basic%20Choice%20Object%20References))
  (Default|ClearOptions (Variables|Default|GetDialogueDisplay))
  (Default|ShowOptions (Variables|Default|GetDialogueDisplay))
  (for (_array_element _array_index) Options
    (if (Variables|/Game/Game/Blueprints/NewDialogueSystem/BP_BasicChoice.BP_BasicChoice_C|GetbCanBeShown? _array_element)
      (Default|AddOption (Variables|Default|GetDialogueDisplay) (Variables|/Game/Game/Blueprints/NewDialogueSystem/BP_BasicChoice.BP_BasicChoice_C|GetChoiceText _array_element) _array_index))))

(fn CreateOption
  (params (bCanBeShown? :type Boolean) (ChoiceID :type Name))
  (bind _returnvalue (Utilities|GetDataTableRow (Variables|Default|GetDialogueChoicesDataTable) ChoiceID)
    (:then
      (bind _returnvalue_2 (Game|ConstructObjectfromClass "/Game/Game/Blueprints/NewDialogueSystem/BP_BasicChoice.BP_BasicChoice_C" bCanBeShown? (Utilities|Struct|BreakST_DialogueOption _returnvalue) ChoiceID))
      (return _returnvalue_2))))

(fn OptionChosen
  (params (IdChosen :type Integer))
  (Default|CallOnOptionChosen IdChosen))

(fn ShowPlayerPortrait
  (params (NewSprite :type Texture%202D%20Object%20Reference))
  (bind _dialoguedisplay (Variables|Default|GetDialogueDisplay))
  (Default|ShowPlayerPortrait _dialoguedisplay NewSprite)
  (Default|HideConversantPortrait _dialoguedisplay))

(fn ShowConversantPortrait
  (params (NewSprite :type Texture%202D%20Object%20Reference))
  (bind _dialoguedisplay (Variables|Default|GetDialogueDisplay))
  (Default|ShowConversantPortrait _dialoguedisplay 0 NewSprite)
  (Default|HidePlayerPortrait _dialoguedisplay))

(fn AddAskedQuestion
  (params (QuestionName :type Name%20%28by%20ref%29))
  (Utilities|Array|AddUnique (Variables|Default|GetAskedQuestions) QuestionName))

(fn ClearAskedQuestions
  (Utilities|Array|Clear (Variables|Default|GetAskedQuestions)))

(fn CheckIsQuestionAsked
  (params (ItemToFind :type Name%20%28by%20ref%29))
  (return (Utilities|Array|ContainsItem (Variables|Default|GetAskedQuestions) ItemToFind)))

(fn CheckAreAllQuestionsAsked
  (params (ArrayName :type Array%20of%20Names))
  (LocalVariables|SetbResult true)
  (bind _array_element (Utilities|Array|ForEachLoopwithBreak ArrayName :!label _label)
    (:LoopBody
      (if (not (CallFunction|CheckIsQuestionAsked _array_element))
        (LocalVariables|SetbResult false)
        (goto _label Break)))
    (:Completed
      (return (LocalVariables|GetbResult)))))

(fn SetCharacterStoryProgression
  (params (CharacterTag :type Gameplay%20Tag%20Structure) (StoryProgressionTag :type Gameplay%20Tag%20Structure))
  (Default|SetCharacterStoryProgression (Variables|Default|GetDAHolder) CharacterTag StoryProgressionTag))

(fn SetThisCharacterStoryProgressionTag
  (params (StoryProgressionTag :type Gameplay%20Tag%20Structure))
  (CallFunction|SetCharacterStoryProgression (Variables|Default|GetCurrentCharacterStatus) StoryProgressionTag))

(fn GetCharacterStoryProgressionTag
  (params (CharacterTag :type Gameplay%20Tag%20Structure))
  (return (Default|GetCharacterStoryProgression (Variables|Default|GetDAHolder) CharacterTag)))

(fn GetThisCharacterStoryProgression
  (return (CallFunction|GetCharacterStoryProgressionTag (Variables|Default|GetCurrentCharacterStatus))))