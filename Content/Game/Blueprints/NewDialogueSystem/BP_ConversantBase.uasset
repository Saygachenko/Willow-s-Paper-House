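; BP_ConversantBase is a base actor for characters the player can talk to, with a sprite and a dialogue component.
; Interacting opens a conversation on the ACBaseDialogue component using the actor's StateTree.
; Hovering the sprite switches the cursor to crosshairs and registers the actor as the player character's interactable message target, clearing both on exit.
; Wrapper functions forward story progression tag getters and setters to the dialogue component.
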(event OnBeginCursorOver(CharacterSprite)
  (params (TouchedComponent :type Primitive%20Component%20Object%20Reference))
  (Variables|/Script/Engine.PlayerController|SetCurrentMouseCursor (Game|GetPlayerController 0) "Crosshairs")
  (Class|BPIMainCharacter|SetInteractable(Message) (Game|GetPlayerCharacter 0) self))

(event OnEndCursorOver(CharacterSprite)
  (params (TouchedComponent :type Primitive%20Component%20Object%20Reference))
  (Variables|/Script/Engine.PlayerController|SetCurrentMouseCursor (Game|GetPlayerController 0) "Default")
  (Class|BPIMainCharacter|ClearInteractable(Message) (Game|GetPlayerCharacter 0)))

(event EventInteract
  (params (Instigator :type Actor%20Object%20Reference))
  (Default|OpenConversation (Variables|Default|GetAC_BaseDialogue) (Variables|Default|GetStateTree)))

(fn ConstructionScript)

(fn SetThisCharacterStoryProgressionTag
  (params (StoryProgressionTag :type Gameplay%20Tag%20Structure))
  (Default|SetThisCharacterStoryProgressionTag (Variables|Default|GetAC_BaseDialogue) StoryProgressionTag))

(fn GetCharacterStoryProgressionTag
  (params (CharacterTag :type Gameplay%20Tag%20Structure))
  (return (Default|GetCharacterStoryProgressionTag (Variables|Default|GetAC_BaseDialogue) CharacterTag)))

(fn GetThisCharacterStoryProgressionTag
  (return (Default|GetThisCharacterStoryProgression (Variables|Default|GetAC_BaseDialogue))))