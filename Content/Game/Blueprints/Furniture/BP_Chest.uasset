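; BP_Chest is an interactable chest that hands a configured item to the player through dialogue.
; On BeginPlay it copies ItemToGive into its DataItemComponent and listens for dialogue events.
; Interact stores the instigator as the player and opens the conversation.
; A "PickUp" dialogue trigger sends the item component to the player's inventory, then unbinds all listeners from that event.
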(event Custom|AddToInventory
  (params (DialogueTrigger :type Name))
  (if (== DialogueTrigger "PickUp")
    (Class|BPIMainCharacter|AddtoInventory(Message) (Variables|Default|GetPlayer) (Variables|Default|GetDataItemComponent))
    (EventDispatchers|UnbindallEventsfromOnDialogueEventTriggered (Variables|Default|GetAC_DialogueBase))))

(event EventBeginPlay
  (Variables|/Game/Game/Blueprints/Components/BP_DataItemComponent.BP_DataItemComponent_C|SetDataItem (Variables|Default|GetDataItemComponent) (Variables|Default|GetItemToGive))
  (EventDispatchers|BindEventtoOnDialogueEventTriggered (Variables|Default|GetAC_DialogueBase) (delegate Custom|AddToInventory)))

(event EventInteract
  (params (Instigator :type Actor%20Object%20Reference))
  (bind _output_get (Variables|Default|SetPlayer Instigator))
  (Default|OpenConveration (Variables|Default|GetAC_DialogueBase) 0.05 _output_get))

(fn ConstructionScript
  (|CallParentFunction))