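; Clickable area over the big clock that runs an item puzzle and reveals a hidden key.
; Using qitem_0006 adds the clock arrow, provided the player also holds qitem_0007; wrong order or missing conditions open dialogue rows.
; With the arrow added and photo seen, using qitem_0007 or plain interaction adds the photo, shows the key and destroys this actor.
; Cursor hover sets or clears the player's interactable message.
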(event OnBeginCursorOver(PaperSprite)
  (params (TouchedComponent :type Primitive%20Component%20Object%20Reference))
  (Class|BPIMainCharacter|SetInteractable(Message) (Game|GetPlayerCharacter 0) self))

(event OnEndCursorOver(PaperSprite)
  (params (TouchedComponent :type Primitive%20Component%20Object%20Reference))
  (Class|BPIMainCharacter|ClearInteractable(Message) (Game|GetPlayerCharacter 0)))

(event Custom|Open
  (Default|AddPhoto (Variables|Default|GetBigClock))
  (Development|SetHiddeninGame (Variables|/Game/Game/Blueprints/Furniture/BP_PickUpSprite.BP_PickUpSprite_C|GetPaperSprite (Variables|Default|GetKey)) false true)
  (Class|BPIMainCharacter|RemovefromInventory(Message) (Game|GetPlayerCharacter 0) "qitem_0007" false)
  (Actor|DestroyActor))

(event EventInteract
  (params (Instigator :type Actor%20Object%20Reference))
  (bind _ac_dialoguebase (Variables|Default|GetAC_DialogueBase))
  (bind _ac_dialoguebase_2 (Variables|Default|GetAC_DialogueBase))
  (bind _ac_dialoguebase_3 (Variables|Default|GetAC_DialogueBase))
  (bind _asbp_main_character (Utilities|Casting|CastToBP_MainCharacter Instigator))
  (if (Variables|/Game/Game/Blueprints/MainCharacter/BP_MainCharacter.BP_MainCharacter_C|GetbIsUsingItem? _asbp_main_character)
    (if (== (Variables|/Game/Game/Blueprints/Components/BP_InventoryComponent.BP_InventoryComponent_C|GetUsingItemID (Variables|/Game/Game/Blueprints/MainCharacter/BP_MainCharacter.BP_MainCharacter_C|GetBP_InventoryComponent _asbp_main_character)) "qitem_0006")
      (bind _isininventory (Default|FindItem (Variables|/Game/Game/Blueprints/MainCharacter/BP_MainCharacter.BP_MainCharacter_C|GetBP_InventoryComponent _asbp_main_character) "qitem_0007"))
      (if _isininventory
        (Default|InteractSuccess _asbp_main_character)
        (Default|AddArrow (Variables|Default|GetBigClock))
        (Variables|Default|SetbArrowAdded? true)
        (Class|BPIMainCharacter|RemovefromInventory(Message) (Game|GetPlayerCharacter 0) "qitem_0006" false)
        (else
          (Variables|/Game/Game/Blueprints/Components/AC_DialogueBase.AC_DialogueBase_C|SetStartingRowName _ac_dialoguebase_3 "20")
          (Default|OpenConveration _ac_dialoguebase_3 0.05 _asbp_main_character)))
      (elif (== (Variables|/Game/Game/Blueprints/Components/BP_InventoryComponent.BP_InventoryComponent_C|GetUsingItemID (Variables|/Game/Game/Blueprints/MainCharacter/BP_MainCharacter.BP_MainCharacter_C|GetBP_InventoryComponent _asbp_main_character)) "qitem_0007")
        (if (Variables|Default|GetbArrowAdded?)
          (if (Variables|/Game/Game/Blueprints/MainCharacter/BP_MainCharacter.BP_MainCharacter_C|GetbSeenPhoto? _asbp_main_character)
            (Default|InteractSuccess _asbp_main_character)
            (CallFunction|Open)
            (else
              (Variables|/Game/Game/Blueprints/Components/AC_DialogueBase.AC_DialogueBase_C|SetStartingRowName _ac_dialoguebase_2 "22")
              (Default|OpenConveration _ac_dialoguebase_2 0.05 _asbp_main_character)))
          (else
            (Variables|/Game/Game/Blueprints/Components/AC_DialogueBase.AC_DialogueBase_C|SetStartingRowName _ac_dialoguebase "21")
            (Default|OpenConveration _ac_dialoguebase 0.05 _asbp_main_character)))))
    (elif (and (Variables|Default|GetbArrowAdded?) (Variables|/Game/Game/Blueprints/MainCharacter/BP_MainCharacter.BP_MainCharacter_C|GetbSeenPhoto? _asbp_main_character))
      (CallFunction|Open))))

(fn ConstructionScript)